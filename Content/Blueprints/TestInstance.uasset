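; TestInstance is a game instance Blueprint that holds the maximum score and persists it between sessions.
; On Init it loads the ScoreSave object from the ScoreSaveData slot and copies its value into MaxScore, leaving it untouched if the cast fails.
; SaveScore writes MaxScore into a newly created ScoreSave and saves it asynchronously to the same slot, while loading is synchronous.
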(event Custom|LoadScore
  (bind _returnvalue (SaveGame|LoadGamefromSlot "ScoreSaveData"))
  (bind _asscore_save (Utilities|Casting|CastToScoreSave _returnvalue))
  (Variables|Default|SetMaxScore (Variables|/Game/Blueprints/Score/ScoreSave.ScoreSave_C|GetScoreValue _asscore_save)))

(event Custom|SaveScore
  (bind _returnvalue (SaveGame|CreateSaveGameObject "/Game/Blueprints/Score/ScoreSave.ScoreSave_C"))
  (Variables|/Game/Blueprints/Score/ScoreSave.ScoreSave_C|SetScoreValue _returnvalue (Variables|Default|GetMaxScore))
  (|AsyncSaveGametoSlot _returnvalue "ScoreSaveData"))

(event EventInit
  (CallFunction|LoadScore))