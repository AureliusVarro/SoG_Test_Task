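; Gameplay ability that fires the side-scroller hero's shotgun when the weapon has clip ammo.
; The montage's Fire notify launches five pellets, then decrements clip ammo and updates the HUD.
; Each pellet randomizes pitch within aim or hip spread, spawns a Niagara tracer and line-traces from the muzzle along the facing direction.
; Trace hits are returned but unused, so no damage is applied here.
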(event Ability|EventActivateAbility
  (bind _weaponref (Variables|Default|GetWeaponRef))
  (Utilities|SetReferences)
  (if (>= (Class|TPWeaponBase|GetClipAmmo (Variables|Default|GetWeaponRef)) 1)
    (bind _notifyname (Animation|Montage|PlayMontage (Variables|/Script/Engine.Character|GetMesh (Variables|Default|GetHeroRef)) "/Game/Assets/Hero/Animations/Hero_Fire_Shotgun_Hip_Montage.Hero_Fire_Shotgun_Hip_Montage" 1.0 0.0 "")
      (:OnCompleted
        (Ability|EndAbility :!label _label))
      (:OnInterrupted
        (goto _label))
      (:OnNotifyBegin
        (if (Utilities|Name|Equal(Name) _notifyname "Fire")
          (for _index (range 0 4)
            (CallFunction|Fire))
          (Class|TPWeaponBase|SetClipAmmo _weaponref (- (Class|TPWeaponBase|GetClipAmmo _weaponref) 1))
          (Default|UpdateAmmo (Variables|/Game/Blueprints/Hero/SideScrollerCharacter.SideScrollerCharacter_C|GetHUD_Ref (Variables|Default|GetHeroRef)) (Variables|Default|GetWeaponRef)))))
    (else
      (Ability|EndAbility))))

(event Ability|EventOnEndAbility
  (params (bWasCancelled :type Boolean)))

(fn Fire
  (bind _weaponref (Variables|Default|GetWeaponRef))
  (LocalVariables|SetWeaponSocketLocation (.location (Transformation|GetSocketTransform (Class|TPWeaponBase|GetMesh _weaponref) (Variables|/Script/TestProject.TP_WeaponBase|GetMuzzleSocket _weaponref) "RTS_World")))
  (LocalVariables|SetSpreadNormalVector (Math|Vector|GetForwardVector (Math|Rotator|MakeRotator 0.0 (CallFunction|GetSpreadOffset) (* (Variables|/Game/Blueprints/Hero/SideScrollerCharacter.SideScrollerCharacter_C|GetDirection (Variables|Default|GetHeroRef)) -9e+01))))
  ;[1 1 1] Spawn laser FX
  (bind _returnvalue (Niagara|SpawnSystematLocation "/Game/Assets/VFX/NS_BulletTrace.NS_BulletTrace" (LocalVariables|GetWeaponSocketLocation)))
  ;;[1 1 1] Set laser speed
  (Effects|Components|ParticleSystem|SetVectorParameter _returnvalue "LaserSpeed" (* (LocalVariables|GetSpreadNormalVector) 2e+03))
  ;[1 1 1] Draw a tracing line
  (bind (_outhit _returnvalue_2) (Collision|LineTraceByChannel (LocalVariables|GetWeaponSocketLocation) (+ (* (LocalVariables|GetSpreadNormalVector) 6e+02) (LocalVariables|GetWeaponSocketLocation)) "TraceTypeQuery1" false 0 "None" true "(R=1.000000,G=0.000000,B=0.000000,A=1.000000)" "(R=0.000000,G=1.000000,B=0.000000,A=1.000000)" 1.0))
  (return _outhit _returnvalue_2))

(fn GetSpreadOffset
  (bind _weaponref (Variables|Default|GetWeaponRef))
  (bind _hipspreadangle (Variables|/Script/TestProject.TP_WeaponBase|GetHipSpreadAngle _weaponref))
  (bind _aimspreadangle (Variables|/Script/TestProject.TP_WeaponBase|GetAimSpreadAngle _weaponref))
  (bind _returnvalue (/ _hipspreadangle 2.0))
  (bind _returnvalue_2 (/ _aimspreadangle 2.0))
  (return (Math|Float|SelectFloat (Math|Random|RandomFloatinRange (* _returnvalue_2 -1.0) _returnvalue_2) (Math|Random|RandomFloatinRange (* _returnvalue -1.0) _returnvalue) (Variables|Default|GetisAiming))))