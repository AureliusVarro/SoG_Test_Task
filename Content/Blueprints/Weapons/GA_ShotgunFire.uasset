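; Gameplay ability for firing the hero's shotgun, which ends immediately if the clip is empty.
; It plays weapon and hero fire animations, and the montage's "Fire" notify triggers several traced pellet shots.
; Hits on BP_Alpha actors apply a damage effect via SetByCaller magnitude and send a knockback event with hit data.
; The notify also spends one round and updates the HUD, and the ability ends when the montage completes or is interrupted.
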(event Ability|EventActivateAbility
  (bind _weaponref (Variables|Default|GetWeaponRef))
  (|CallParentFunction)
  (if (>= (Class|TPWeaponBase|GetClipAmmo (Variables|Default|GetWeaponRef)) 1)
    (Components|Animation|PlayAnimation (Class|TPWeaponBase|GetMesh (Variables|Default|GetWeaponRef)) "/Game/SciFiWeapDark/Weapons/Anims/Fire_Shotgun_W.Fire_Shotgun_W" false)
    (bind _notifyname (Animation|Montage|PlayMontage (Variables|/Script/Engine.Character|GetMesh (Variables|Default|GetHeroRef)) "/Game/Assets/Hero/Animations/Hero_Fire_Shotgun_Hip_Montage.Hero_Fire_Shotgun_Hip_Montage" 1.0 0.0 "")
      (:OnCompleted
        (Ability|EndAbility :!label _label))
      (:OnInterrupted
        (goto _label))
      (:OnNotifyBegin
        (if (Utilities|Name|Equal(Name) _notifyname "Fire")
          (for _index (range 0 4)
            (bind (_outhit _returnvalue) (CallFunction|Fire))
            (if _returnvalue
              (bind _asbp_alpha (Utilities|Casting|CastToBP_Alpha (.HitActor (Collision|BreakHitResult _outhit))))
              (bind _returnvalue_2 (Ability|GameplayEffect|AssignTagSetbyCallerMagnitude (Ability|MakeOutgoingGameplayEffectSpec (Variables|Default|GetDamageGameplayEffectClass) (Math|Conversions|ToFloat(Integer) (Ability|GetAbilityLevel))) "(TagName=\"Data.Damage\")" (Variables|Default|GetDamage)))
              (GameplayEffects|ApplyGameplayEffectSpecToTarget (Ability|GetAbilitySystemComponent _asbp_alpha) _returnvalue_2 (Ability|GetAbilitySystemComponent _asbp_alpha))
              (Ability|SendGameplayEventtoActor (.HitActor (Collision|BreakHitResult _outhit)) "(TagName=\"Event.knockback\")" (Utilities|Struct|MakeGameplayEventData "" 0 0 0 0 "()" "(GameplayTags=)" "(GameplayTags=)" 0.0 (Ability|TargetData|AbilityTargetDatafromHitResult _outhit)))))
          (Class|TPWeaponBase|SetClipAmmo _weaponref (- (Class|TPWeaponBase|GetClipAmmo _weaponref) 1))
          (Default|UpdateAmmo (Variables|/Game/Blueprints/Hero/SideScrollerCharacter.SideScrollerCharacter_C|GetHUD_Ref (Variables|Default|GetHeroRef)) (Variables|Default|GetWeaponRef)))))
    (else
      (Ability|EndAbility))))