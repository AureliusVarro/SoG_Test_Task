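; Base gameplay ability for side-scroller weapon fire, providing a Fire function that returns a hit result.
; Activation caches the character and source weapon, ending if either cast fails.
; Fire applies aim or hip random spread to the vertical aim, constrained to the facing direction.
; It spawns a velocity-compensated Niagara laser at the muzzle, shakes the camera and line-traces for Pawns, leaving hit handling outside this file.
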(event Ability|EventActivateAbility
  (bind _asside_scroller_character (Utilities|Casting|CastToSideScrollerCharacter (Ability|GetAvatarActorfromActorInfo))
    (:then
      (Variables|Default|SetHeroRef _asside_scroller_character)
      (bind _astp_weapon_base (Utilities|Casting|CastToTP_WeaponBase (Ability|GetCurrentSourceObject))
        (:then
          (Variables|Default|SetWeaponRef _astp_weapon_base))
        (:CastFailed
          (Ability|EndAbility :!label _label))))
    (:CastFailed
      (goto _label))))

(event Ability|EventOnEndAbility
  (params (bWasCancelled :type Boolean)))

(fn GetSpreadOffset
  (bind _weaponref (Variables|Default|GetWeaponRef))
  (bind _hipspreadangle (Variables|/Script/TestProject.TP_WeaponBase|GetHipSpreadAngle _weaponref))
  (bind _aimspreadangle (Variables|/Script/TestProject.TP_WeaponBase|GetAimSpreadAngle _weaponref))
  (bind _returnvalue (/ _hipspreadangle 2.0))
  (bind _returnvalue_2 (/ _aimspreadangle 2.0))
  (return (Math|Float|SelectFloat (Math|Random|RandomFloatinRange (* _returnvalue_2 -1.0) _returnvalue_2) (Math|Random|RandomFloatinRange (* _returnvalue -1.0) _returnvalue) (Variables|/Game/Blueprints/Hero/SideScrollerCharacter.SideScrollerCharacter_C|GetAiming (Variables|Default|GetHeroRef)))))

(fn Fire
  (bind _weaponref (Variables|Default|GetWeaponRef))
  (LocalVariables|SetWeaponSocketLocation (Transformation|GetSocketLocation (Class|TPWeaponBase|GetMesh _weaponref) (Variables|/Script/TestProject.TP_WeaponBase|GetMuzzleSocket _weaponref)))
  (LocalVariables|SetSpreadNormalVector (Math|Vector|GetForwardVector (Math|Rotator|MakeRotator 0.0 (- (CallFunction|GetSpreadOffset) (* (Variables|/Game/Blueprints/Hero/SideScrollerCharacter.SideScrollerCharacter_C|GetAimOffsetVertical (Variables|Default|GetHeroRef)) -1.0)) (* (Variables|/Game/Blueprints/Hero/SideScrollerCharacter.SideScrollerCharacter_C|GetDirection (Variables|Default|GetHeroRef)) -9e+01))))
  ;[1 1 1] Spawn laser FX
  (bind _returnvalue (Niagara|SpawnSystematLocation "/Game/Assets/VFX/NS_BulletTrace.NS_BulletTrace" (+ (LocalVariables|GetWeaponSocketLocation) (* (Transformation|GetVelocity (Variables|Default|GetHeroRef)) (* (Utilities|Time|GetWorldDeltaSeconds) 1e+01)))))
  (Camera|PlayWorldCameraShake (Variables|Default|GetCameraShake) (Camera|GetCameraLocation (Game|GetPlayerCameraManager 0)) 0.0 3e+02)
  ;;[1 1 1] Set laser speed
  (Effects|Components|ParticleSystem|SetVectorParameter _returnvalue "LaserSpeed" (* (LocalVariables|GetSpreadNormalVector) 2.5e+03))
  ;[1 1 1] Draw a tracing line
  (bind (_outhit _returnvalue_2) (Collision|LineTraceForObjects (LocalVariables|GetWeaponSocketLocation) (+ (* (LocalVariables|GetSpreadNormalVector) 1.8e+03) (LocalVariables|GetWeaponSocketLocation)) (Utilities|Array|MakeArray "ObjectTypeQuery3") false 0 "None"))
  (return _outhit _returnvalue_2))