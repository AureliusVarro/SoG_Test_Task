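; Wave spawner for the side-scroller that spawns escalating waves of BP_EnemyAlphaa once the game mode signals game start.
; A looped spawn fills each wave at random BP_SpawnPoint boxes, randomizing Y and lifting Z slightly.
; Each enemy's destroyed event decrements the alive count, which a self-repeating one-second check watches to start the next wave.
; Wave size equals the wave number early on, then becomes a random range around it.
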(event Custom|CheckEnemyAlive
  ;[1 1 1] Check each second if all enemies are dead, then start new wave
  (Utilities|FlowControl|Delay 1.0)
  (if (<= (Variables|Default|GetEnemyAlive) 0)
    (Math|Integer|IncrementInt (Variables|Default|GetWaveNumber)
      (:%20%20
        (Variables|Default|SetEnemyForThisWave (CallFunction|EnemyforCurrentWave))
        (Variables|Default|SetSpawnedEnemies 0)
        (CallFunction|StartNewWave)))
    (else
      (CallFunction|CheckEnemyAlive))))

(event Custom|StartNewWave
  (bind _returnvalue (Game|SpawnActorfromClass "/Game/Blueprints/Enemy/BP_EnemyAlphaa.BP_EnemyAlphaa_C" (Math|Transform|MakeTransform (.SpawnPointLocation (CallFunction|GetRandomSpawnPoint)) "0, 0, 0" "1,1,1") "AdjustIfPossibleButAlwaysSpawn" 0 0 :!label _label))
  (EventDispatchers|BindEventtoEnemyDestoyed _returnvalue (delegate Custom|DecrenentEnemyAlive))
  (Pawn|SpawnDefaultController _returnvalue)
  (bind _result (Math|Integer|IncrementInt (Variables|Default|GetSpawnedEnemies))
    (:%20%20
      (Math|Integer|IncrementInt (Variables|Default|GetEnemyAlive)
        (:%20%20
          (if (== (Variables|Default|GetEnemyForThisWave) _result)
            ;[1 1 1] Check each second if all enemies are dead, then start new wave
            (if (<= (Variables|Default|GetEnemyAlive) 0)
              (Math|Integer|IncrementInt (Variables|Default|GetWaveNumber)
                (:%20%20
                  (Variables|Default|SetEnemyForThisWave (CallFunction|EnemyforCurrentWave))
                  (Variables|Default|SetSpawnedEnemies 0)
                  (CallFunction|StartNewWave)))
              (else
                (CallFunction|CheckEnemyAlive)))
            (else
              (goto _label))))))))

(event Custom|OnGameStarted_Event_0
  (bind _returnvalue (Game|SpawnActorfromClass "/Game/Blueprints/Enemy/BP_EnemyAlphaa.BP_EnemyAlphaa_C" (Math|Transform|MakeTransform (.SpawnPointLocation (CallFunction|GetRandomSpawnPoint)) "0, 0, 0" "1,1,1") "AdjustIfPossibleButAlwaysSpawn" 0 0 :!label _label))
  (EventDispatchers|BindEventtoEnemyDestoyed _returnvalue (delegate Custom|DecrenentEnemyAlive))
  (Pawn|SpawnDefaultController _returnvalue)
  (bind _result (Math|Integer|IncrementInt (Variables|Default|GetSpawnedEnemies))
    (:%20%20
      (Math|Integer|IncrementInt (Variables|Default|GetEnemyAlive)
        (:%20%20
          (if (== (Variables|Default|GetEnemyForThisWave) _result)
            ;[1 1 1] Check each second if all enemies are dead, then start new wave
            (if (<= (Variables|Default|GetEnemyAlive) 0)
              (Math|Integer|IncrementInt (Variables|Default|GetWaveNumber)
                (:%20%20
                  (Variables|Default|SetEnemyForThisWave (CallFunction|EnemyforCurrentWave))
                  (Variables|Default|SetSpawnedEnemies 0)
                  (CallFunction|StartNewWave)))
              (else
                (CallFunction|CheckEnemyAlive)))
            (else
              (goto _label))))))))

(event Custom|DecrenentEnemyAlive
  ;[1 1 1] Value of enemies on level
  ; decrement when enemy killed
  (Math|Integer|DecrementInt (Variables|Default|GetEnemyAlive)))

(event EventBeginPlay
  (EventDispatchers|AssignOnGameStarted (.AsSide%20Scroller%20Game%20Mode (Utilities|Casting|CastToSideScrollerGameMode (Game|GetGameMode))) (delegate Custom|OnGameStarted_Event_0)))

(event Collision|EventActorBeginOverlap
  (params (OtherActor :type Actor%20Object%20Reference)))

(fn ConstructionScript)

(fn GetRandomSpawnPoint
  (bind _outactors (Actor|GetAllActorsOfClass "/Game/Blueprints/Enemy/BP_SpawnPoint.BP_SpawnPoint_C"))
  (bind _output_get (Variables|Default|SetSpawnPointRef (Utilities|Array|Get(acopy) _outactors (Math|Random|RandomIntegerinRange 0 (Utilities|Array|LastIndex _outactors)))))
  (bind _output_get_2 (Variables|Default|SetSpawnPointLocation (Math|Random|RandomPointinBoundingBox (Math|Vector|MakeVector 0.0 (.y (.location (Transformation|GetWorldTransform (Variables|/Game/Blueprints/Enemy/BP_SpawnPoint.BP_SpawnPoint_C|GetBox (Utilities|Array|Get(acopy) _outactors (Math|Random|RandomIntegerinRange 0 (Utilities|Array|LastIndex _outactors))))))) 0.0) (Components|Box|GetScaledBoxExtent (Variables|/Game/Blueprints/Enemy/BP_SpawnPoint.BP_SpawnPoint_C|GetBox (Utilities|Array|Get(acopy) _outactors (Math|Random|RandomIntegerinRange 0 (Utilities|Array|LastIndex _outactors))))))))
  (return true (Math|Vector|MakeVector (.x (.location (Transformation|GetWorldTransform (Variables|/Game/Blueprints/Enemy/BP_SpawnPoint.BP_SpawnPoint_C|GetBox (Utilities|Array|Get(acopy) _outactors (Math|Random|RandomIntegerinRange 0 (Utilities|Array|LastIndex _outactors))))))) (.y _output_get_2) (+ (.z (.location (Transformation|GetWorldTransform (Variables|/Game/Blueprints/Enemy/BP_SpawnPoint.BP_SpawnPoint_C|GetBox (Utilities|Array|Get(acopy) _outactors (Math|Random|RandomIntegerinRange 0 (Utilities|Array|LastIndex _outactors))))))) 3e+01)) _output_get))

(fn EnemyforCurrentWave
  (bind _wavenumber (Variables|Default|GetWaveNumber))
  (bind _wavenumber_2 (Variables|Default|GetWaveNumber))
  (if (<= _wavenumber_2 3)
    (bind _output_get (Variables|Default|SetEnemyForThisWave _wavenumber_2))
    (return _output_get)
    (else
      (bind _output_get_2 (Variables|Default|SetEnemyForThisWave (Math|Random|RandomIntegerinRange (- _wavenumber 3) (+ _wavenumber 5))))
      (return _output_get_2))))