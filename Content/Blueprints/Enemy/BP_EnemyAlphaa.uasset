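; Enemy actor that announces its destruction through an EnemyDestoyed call.
; On BeginPlay it waits briefly, makes that call and destroys itself, with no further condition.
; Death_Event switches the capsule to physics-only collision and launches the physics-simulated static mesh with a random velocity-change impulse.
; After a short delay, that event destroys the actor and makes the same call.
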(event Custom|Death_Event
  (Collision|SetCollisionEnabled (Variables|Default|GetCapsuleComponent) "PhysicsOnly")
  (Physics|SetSimulatePhysics (Variables|Default|GetStaticMesh) true)
  (Physics|AddImpulse (Variables|Default|GetStaticMesh) (Math|Vector|MakeVector (Math|Random|RandomFloatinRange -1e+03 3e+03) (Math|Random|RandomFloatinRange -1e+03 1e+03) (Math|Random|RandomFloatinRange 1e+01 1e+02)) "None" true)
  (Utilities|FlowControl|Delay 1.0)
  (Actor|DestroyActor)
  (Development|PrintString "destroyed")
  (Default|CallEnemyDestoyed))

(event EventBeginPlay
  (Utilities|FlowControl|Delay 2.0)
  (Default|CallEnemyDestoyed)
  (Actor|DestroyActor)
  (Development|PrintString "event called"))

(fn ConstructionScript)