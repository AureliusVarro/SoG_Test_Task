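; AI_Enemy2 is an enemy character Blueprint that handles its own death and a timed size change.
; On death it disables movement and capsule collision, turns the mesh into a partially blended physics ragdoll with an impulse, then destroys itself after a delay.
; The size-change event drives actor scale from a Timeline, then calls StopChangeSizeEvent1 when the Timeline finishes.
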(event Custom|StartChageSizeEvent_Event
  (bind _returnvalue (Transformation|GetActorTransform))
  ;[1 1 1] Change size actor
  (Development|PrintString "StartChange")
  (bind _newtrack_0 (Timeline|Timeline_1 Play)
    (:Update
      (Transformation|SetActorTransform (Math|Transform|MakeTransform (.location _returnvalue) (.rotation _returnvalue) _newtrack_0) false true))
    (:Finished
      (Default|CallStopChangeSizeEvent1))))

(event Custom|DeathEvent_Event
  (Pawn|Components|CharacterMovement|DisableMovement (Variables|Character|GetCharacterMovement))
  (Collision|SetCollisionEnabled (Variables|Default|GetCapsuleComponent) "NoCollision")
  (Class|SkeletalMeshComponent|SetAllBodiesSimulatePhysics (Variables|Character|GetMesh) true)
  (Class|SkeletalMeshComponent|SetAllBodiesPhysicsBlendWeight (Variables|Character|GetMesh) 0.1 false)
  (Physics|AddImpulse (Variables|Character|GetMesh) "4.000000,15.000000,6.000000" "None" true)
  (Utilities|FlowControl|Delay 5.0)
  (Actor|DestroyActor))

(event Collision|EventActorBeginOverlap
  (params (OtherActor :type Actor%20Object%20Reference)))

(fn ConstructionScript)