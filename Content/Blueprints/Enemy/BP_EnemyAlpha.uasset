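; BP_EnemyAlpha is an enemy Blueprint whose graph handles only its death.
; On the death event it turns off capsule collision, enables physics on its static mesh and flings it with a random, mass-independent velocity impulse biased toward positive X.
; After a short delay the actor destroys itself.
; A DisableMovement call on the character movement component is left unconnected and never runs.
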(event Custom|DeathEvent_Event
  (Collision|SetCollisionEnabled (Variables|Default|GetCapsuleComponent) "NoCollision")
  (Physics|SetSimulatePhysics (Variables|Default|GetStaticMesh) true)
  (Physics|AddImpulse (Variables|Default|GetStaticMesh) (Math|Vector|MakeVector (Math|Random|RandomFloatinRange -1e+03 3e+03) (Math|Random|RandomFloatinRange -1e+03 1e+03) (Math|Random|RandomFloatinRange 1e+01 1e+02)) "None" true)
  (Utilities|FlowControl|Delay 5.0)
  (Actor|DestroyActor))

(fn ConstructionScript)