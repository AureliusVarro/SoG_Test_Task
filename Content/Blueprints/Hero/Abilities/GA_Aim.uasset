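; Gameplay ability that lets the side-scroller hero aim with the mouse while input is held.
; Activation halves walk speed, sets the aiming flag and shows the cursor; release ends it and restores these.
; A frame-delta WaitDelay loop turns the screen-space hand-to-cursor vector into vertical aim offset, ignoring cursors too close.
; Angles are relative to facing, with an optional mirrored check for aiming behind.
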(event Ability|EventActivateAbility
  (bind _mindistance (Variables|Default|GetMinDistance))
  (bind (_can _direction_vector) (Utilities|GetDirVector _mindistance))
  (bind _asside_scroller_character (Utilities|Casting|CastToSideScrollerCharacter (Ability|GetOwningActorfromActorInfo))
    (:then
      (bind _output_get (Variables|Default|SetStartSpeed (Class|MovementComponent|GetMaxSpeed (Variables|/Script/Engine.Character|GetCharacterMovement _asside_scroller_character))))
      (Variables|/Script/Engine.CharacterMovementComponent|SetMaxWalkSpeed (Variables|/Script/Engine.Character|GetCharacterMovement _asside_scroller_character) (/ _output_get 2.0))
      (bind _output_get_2 (Variables|Default|SetHeroREF _asside_scroller_character))
      (Variables|/Game/Blueprints/Hero/SideScrollerCharacter.SideScrollerCharacter_C|SetAiming _output_get_2 true)
      (bind _output_get_3 (Variables|Default|SetControllerREF (Game|GetPlayerController 0)))
      (Variables|/Script/Engine.PlayerController|SetbShowMouseCursor _output_get_3 true)
      (Ability|Tasks|WaitInputRelease false
        (:then
          (Ability|Tasks|WaitDelay (Utilities|Time|GetWorldDeltaSeconds) :!label _label
            (:OnFinish
              (if _can
                (if (and (< (Utilities|CheckAngle (Variables|/Game/Blueprints/Hero/SideScrollerCharacter.SideScrollerCharacter_C|GetDirection (Variables|Default|GetHeroREF)) _direction_vector) 9e+01) (> (Utilities|CheckAngle (Variables|/Game/Blueprints/Hero/SideScrollerCharacter.SideScrollerCharacter_C|GetDirection (Variables|Default|GetHeroREF)) _direction_vector) -9e+01))
                  (Variables|/Game/Blueprints/Hero/SideScrollerCharacter.SideScrollerCharacter_C|SetAimOffsetVertical (Variables|Default|GetHeroREF) (Utilities|CheckAngle (Variables|/Game/Blueprints/Hero/SideScrollerCharacter.SideScrollerCharacter_C|GetDirection (Variables|Default|GetHeroREF)) _direction_vector))
                  (goto _label)
                  (elif (Variables|Default|GetCkeckInBack)
                    (Variables|/Game/Blueprints/Hero/SideScrollerCharacter.SideScrollerCharacter_C|SetAimOffsetVertical (Variables|Default|GetHeroREF) (Utilities|CheckAngle (* (Variables|/Game/Blueprints/Hero/SideScrollerCharacter.SideScrollerCharacter_C|GetDirection (Variables|Default|GetHeroREF)) -1) _direction_vector))
                    (goto _label)
                    (else
                      (goto _label))))
                (else
                  (goto _label))))))
        (:OnRelease
          (Ability|EndAbility))))
    (:CastFailed
      (Ability|EndAbility))))

(event Ability|EventOnEndAbility
  (params (bWasCancelled :type Boolean))
  (bind _heroref (Variables|Default|GetHeroREF))
  (Variables|/Game/Blueprints/Hero/SideScrollerCharacter.SideScrollerCharacter_C|SetAiming _heroref false)
  (Variables|/Game/Blueprints/Hero/SideScrollerCharacter.SideScrollerCharacter_C|SetAimOffsetVertical _heroref 0.0)
  (Variables|/Script/Engine.CharacterMovementComponent|SetMaxWalkSpeed (Variables|/Script/Engine.Character|GetCharacterMovement _heroref) (Variables|Default|GetStartSpeed))
  (Variables|/Script/Engine.PlayerController|SetbShowMouseCursor (Variables|Default|GetControllerREF) false))