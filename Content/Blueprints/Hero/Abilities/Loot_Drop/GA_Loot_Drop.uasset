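; Gameplay ability that rolls a random loot drop, apparently for enemies.
; On activation, a 1–100 roll picks armor, health potion, ammo, one of three timed-style bonuses (flash, immortality, infinite ammo) or nothing, then ends.
; LootDropImpulse spawns the pickup at the instigator's location and launches its mesh along the instigator's up vector, randomly tilted within angle limits.
; Only the armor branch explicitly passes the owner as instigator.
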(event Ability|EventActivateAbility
  (Variables|Default|SetRandomValue (Math|Random|RandomIntegerinRange 1 100))
  ;[1 1 1] System of loot drop
  (if (<= (Variables|Default|GetRandomValue) 5)
    ;[1 1 1] Armor
    (CallFunction|LootDropImpulse "/Game/Blueprints/Hero/Abilities/Pickup/BP_Armor.BP_Armor_C" (.owneractor (Ability|GetActorInfo)))
    (Ability|EndAbility)
    (elif (and (> (Variables|Default|GetRandomValue) 5) (< (Variables|Default|GetRandomValue) 16))
      ;[1 1 1] HP
      (CallFunction|LootDropImpulse "/Game/Blueprints/Hero/Abilities/Pickup/BP_HealthPotion.BP_HealthPotion_C")
      (Ability|EndAbility)
      (elif (and (> (Variables|Default|GetRandomValue) 15) (< (Variables|Default|GetRandomValue) 31))
        ;[1 1 1] Ammo
        (CallFunction|LootDropImpulse "/Game/Blueprints/Hero/Abilities/Pickup/BP_Ammo.BP_Ammo_C")
        (Ability|EndAbility)
        (elif (and (> (Variables|Default|GetRandomValue) 30) (< (Variables|Default|GetRandomValue) 34))
          ;[1 1 1] Flash
          (CallFunction|LootDropImpulse "/Game/Blueprints/Hero/Abilities/Pickup/BP_Bonus_Flash.BP_Bonus_Flash_C")
          (Ability|EndAbility)
          (elif (and (> (Variables|Default|GetRandomValue) 33) (< (Variables|Default|GetRandomValue) 37))
            ;[1 1 1] Immortality
            (CallFunction|LootDropImpulse "/Game/Blueprints/Hero/Abilities/Pickup/BP_Bonus_Immortality.BP_Bonus_Immortality_C")
            (Ability|EndAbility)
            (elif (and (> (Variables|Default|GetRandomValue) 36) (< (Variables|Default|GetRandomValue) 41))
              ;[1 1 1] Infinity Ammo
              (CallFunction|LootDropImpulse "/Game/Blueprints/Hero/Abilities/Pickup/BP_Bonus_InfinityAmmo.BP_Bonus_InfinityAmmo_C")
              (Ability|EndAbility)
              (else
                (Ability|EndAbility)))))))))

(event Ability|EventOnEndAbility
  (params (bWasCancelled :type Boolean)))

(fn LootDropImpulse
  (params (SupplySpawnClass :type Actor%20Class%20Reference) (EnemyDropInstigator :type Actor%20Object%20Reference))
  (bind _returnvalue (Game|SpawnActorfromClass SupplySpawnClass (Math|Transform|MakeTransform (Transformation|GetActorLocation EnemyDropInstigator) "0, 0, 0" "1,1,1") "Undefined" 0 0))
  (bind _asbp_pickupable (Utilities|Casting|CastToBP_Pickupable _returnvalue)
    (:then
      (Physics|AddImpulse (Variables|/Game/Blueprints/Hero/Abilities/Pickup/BP_Pickupable.BP_Pickupable_C|GetMesh _asbp_pickupable) (* (Math|Vector|Normalize (Math|Vector|RotateVector (Math|Vector|GetUpVector (Transformation|GetActorRotation EnemyDropInstigator)) (Math|Rotator|MakeRotator (Math|Random|RandomFloatinRange (* (Variables|Default|GetMax%20Left%20Angle) -1.0) (Variables|Default|GetMax%20Right%20Angle)) 0.0 0.0))) (Variables|Default|GetForce)) "None" true))
    (:CastFailed
      (Ability|EndAbility))))